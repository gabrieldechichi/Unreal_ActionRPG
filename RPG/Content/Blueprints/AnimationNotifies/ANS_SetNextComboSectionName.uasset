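; Anim notify state that opens a combo window on an RPG character's montage.
; On begin, it picks a random name from its ComboSections array and sets it as the character's next combo section.
; On end, it resets that name, so the chosen section applies only during the notify's span.
; The character is resolved from the mesh component, and nothing happens when that lookup is not valid.
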(fn ReceivedNotifyBegin
  (params (MeshComp :type Skeletal%20Mesh%20Component%20Object%20Reference) (Animation :type Anim%20Sequence%20Base%20Object%20Reference) (TotalDuration :type Float%20%28single-precision%29))
  (bind _combosections (Variables|Default|GetComboSections))
  (bind _playercharacter (Utilities|GetRPGCharacterfromMesh MeshComp)
    (:Valid
      (Default|SetNextComboSectionName _playercharacter (Utilities|Array|Get(acopy) _combosections (Math|Random|RandomInteger (Utilities|Array|Length _combosections))))
      (return true))))

(fn ReceivedNotifyEnd
  (params (MeshComp :type Skeletal%20Mesh%20Component%20Object%20Reference) (Animation :type Anim%20Sequence%20Base%20Object%20Reference))
  (bind _playercharacter (Utilities|GetRPGCharacterfromMesh MeshComp)
    (:Valid
      (Default|ResetNextComboSectionName _playercharacter)
      (return true))))