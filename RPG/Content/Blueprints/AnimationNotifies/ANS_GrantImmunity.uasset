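; Animation notify state that makes an RPG character immune for the length of a montage or animation window.
; On begin it finds the character from the mesh, sets IsImmune and applies the ImmunityEffect gameplay effect to its own ability system component.
; On end it clears IsImmune and removes all stacks of that effect, pairing a plain flag with a GAS effect.
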(fn ReceivedNotifyBegin
  (params (MeshComp :type Skeletal%20Mesh%20Component%20Object%20Reference) (Animation :type Anim%20Sequence%20Base%20Object%20Reference) (TotalDuration :type Float%20%28single-precision%29))
  (bind _playercharacter (Utilities|GetRPGCharacterfromMesh MeshComp)
    (:Valid
      (Variables|/Game/RPG/Core/BP_Character.BP_Character_C|SetIsImmune _playercharacter true)
      (GameplayEffects|ApplyGameplayEffectToSelf :self (Ability|GetAbilitySystemComponent _playercharacter) :GameplayEffectClass (Variables|Default|GetImmunityEffect))
      (return true))))

(fn ReceivedNotifyEnd
  (params (MeshComp :type Skeletal%20Mesh%20Component%20Object%20Reference) (Animation :type Anim%20Sequence%20Base%20Object%20Reference))
  (bind _playercharacter (Utilities|GetRPGCharacterfromMesh MeshComp)
    (:Valid
      (Variables|/Game/RPG/Core/BP_Character.BP_Character_C|SetIsImmune _playercharacter false)
      (GameplayEffects|RemoveActiveGameplayEffectbySourceEffect (Ability|GetAbilitySystemComponent _playercharacter) (Variables|Default|GetImmunityEffect) 0 -1)
      (return true))))