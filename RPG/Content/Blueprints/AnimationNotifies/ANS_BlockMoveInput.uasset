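; Anim notify state that blocks the owning pawn's movement input for the span of the notify in an animation.
; On begin and end it casts the mesh owner to Pawn, fetches its RPG player controller and sets the movement input block on, then off.
; A helper function wraps the same controller lookup from a mesh component, though neither event calls it.
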(fn ReceivedNotifyBegin
  (params (MeshComp :type Skeletal%20Mesh%20Component%20Object%20Reference) (Animation :type Anim%20Sequence%20Base%20Object%20Reference) (TotalDuration :type Float%20%28single-precision%29))
  (bind _aspawn (Utilities|Casting|CastToPawn (Components|GetOwner MeshComp)))
  (Default|SetBlockMovementInput (CallFunction|GetRPGPlayerController _aspawn _aspawn) true)
  (return true))

(fn ReceivedNotifyEnd
  (params (MeshComp :type Skeletal%20Mesh%20Component%20Object%20Reference) (Animation :type Anim%20Sequence%20Base%20Object%20Reference))
  (bind _aspawn (Utilities|Casting|CastToPawn (Components|GetOwner MeshComp)))
  (Default|SetBlockMovementInput (CallFunction|GetRPGPlayerController _aspawn _aspawn) false)
  (return true))

(fn GetRPGPlayerControllerfromMesh
  (params (MeshComp :type Mesh%20Component%20Object%20Reference))
  (bind _aspawn (Utilities|Casting|CastToPawn (Components|GetOwner MeshComp)))
  (return (CallFunction|GetRPGPlayerController _aspawn _aspawn)))