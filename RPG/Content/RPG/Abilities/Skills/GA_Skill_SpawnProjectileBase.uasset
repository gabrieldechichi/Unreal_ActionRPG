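; Base gameplay ability for projectile skills: plays a montage and spawns a projectile from the avatar when a gameplay event arrives.
; After committing, it runs PlayMontageAndWaitForEvent, and each received event builds an effect container spec from its tag and data.
; That spec passes to the configurable projectile class, spawned at the avatar pawn's location and rotation with it as instigator.
; Montage blend-out, interruption or cancellation ends the ability.
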(event Ability|EventActivateAbility
  (bind _returnvalue (Ability|CommitAbility))
  (if _returnvalue
    (bind (_asynctaskproxy _eventtag _eventdata) (|PlayMontageandWaitforEvent :MontageToPlay (Variables|Default|GetMontageToPlay))
      (:OnBlendOut
        (Ability|EndAbility :!label _label))
      (:OnInterrupted
        (goto _label))
      (:OnCancelled
        (goto _label))
      (:EventReceived
        (bind _returnvalue_2 (Class|RPGGameplayAbility|MakeEffectContainerSpec _eventtag _eventdata -1))
        (bind _aspawn (Utilities|Casting|CastToPawn (Ability|GetAvatarActorfromActorInfo)))
        (Game|SpawnActorfromClass (Variables|Default|GetProjectilePawn) (Math|Transform|MakeTransform (Transformation|GetActorLocation _aspawn) (Transformation|GetActorRotation _aspawn) "1,1,1") "AlwaysSpawn" 0 _returnvalue_2 _aspawn)))))

(event Ability|EventOnEndAbility
  (params (bWasCancelled :type Boolean)))