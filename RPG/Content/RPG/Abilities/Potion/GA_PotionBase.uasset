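; GA_PotionBase is a base gameplay ability for using potions.
; After committing, it plays a montage, applies its effect container on the shared UseItem montage event, and ends then or when the montage completes, blends out or is stopped.
; CanActivateAbility refuses GA_PotionHealth and its children on authority but allows them on non-authority.
; The server's activation response is printed as a debug string.
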(event Ability|EventActivateAbility
  (bind _returnvalue (Ability|CommitAbility))
  (if _returnvalue
    (|PlayMontageandWaitProxy "None" (Variables|Default|GetMontageToPlay) 1.0 "None" true 1.0
      (:then
        (Ability|Tasks|WaitGameplayEvent "(TagName=\"Event.Montage.Shared.UseItem\")" 0
          (:EventReceived
            (Class|RPGGameplayAbility|ApplyEffectContainer :EventTag "(TagName=\"Event.Montage.Shared.UseItem\")")
            (Ability|EndAbility))))
      (:OnCompleted
        (Ability|EndAbility :!label _label))
      (:OnBlendOut
        (goto _label))
      (:OnInterrupted
        (goto _label))
      (:OnCancelled
        (goto _label)))))

(event EventReceiveServerAbilityActivationResponse
  (params (bAccepted :type Boolean))
  (Development|PrintString (Utilities|String|ToString(Boolean) bAccepted)))

(fn K2CanActivateAbility
  (params (ActorInfo :type Gameplay%20Ability%20Actor%20Info%20Structure))
  (return "" (or (not (Ability|HasAuthority (.OwnerActor (Utilities|Struct|BreakGameplayAbilityActorInfo ActorInfo)))) (not (Utilities|ClassIsChildOf (Utilities|GetClass self) "/Game/RPG/Abilities/Potion/GA_PotionHealth.GA_PotionHealth_C")))))