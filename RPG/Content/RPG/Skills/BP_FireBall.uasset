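; BP_FireBall is a fireball skill actor that explodes on contact with an RPG character.
; On overlap it runs the parent handler, then checks that the other actor derives from RPGCharacterBase and is not its instigator.
; A valid hit spawns the P_Bomb particle effect at the fireball's location and destroys the actor.
; The construction script only calls the parent.
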(event Collision|EventActorBeginOverlap
  (params (OtherActor :type Actor%20Object%20Reference))
  (|CallParentFunction OtherActor)
  (if (and (Utilities|ClassIsChildOf (Utilities|GetClass OtherActor) "/Script/RPG.RPGCharacterBase") (!= OtherActor (Game|GetInstigator)))
    (Effects|SpawnEmitteratLocation "/Game/Effects/FX_Mobile/P_Bomb.P_Bomb" (Transformation|GetActorLocation))
    (Actor|DestroyActor)))

(fn ConstructionScript
  (|CallParentFunction))