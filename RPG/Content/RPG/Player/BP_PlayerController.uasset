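; BP_PlayerController is the RPG player controller that turns input into character movement, camera yaw and HUD display.
; Each Tick, unless movement input is blocked, it moves the possessed BP_PlayerCharacter relative to the camera.
; During melee, input instead lerps the character's rotation toward the camera-relative stick direction at its RotateSpeed.
; On possess, it creates WBP_HUD_PC once and makes it visible.
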(event Custom|CreateHUD
  ;[1 1 1] HUD
  (bind _returnvalue (UserInterface|CreateWidget "/Game/Blueprints/Widgets/WBP_HUD_PC.WBP_HUD_PC_C" self))
  (bind _output_get (Variables|Default|SetPlayerHUD _returnvalue))
  (UserInterface|Viewport|AddtoViewport _output_get 0))

(event Custom|SetHUDVisiblity
  (params (bNewVisible :type Boolean))
  (bind _playerhud (Variables|Default|GetPlayerHUD))
  ;[1 1 1] HUD
  (Utilities|IsValid _playerhud
    (:Is%20Valid
      (Widget|SetVisibility _playerhud (select bNewVisible "SelfHitTestInvisible" "Hidden")))))

(event EventBeginPlay)

(event EventTick
  (params (DeltaSeconds :type Float%20%28single-precision%29))
  (if (Movement|ShouldProcessMovement)
    (bind _character (Utilities|GetValidControlledCharacter)
      (:Valid
        (if (Default|IsUsingMelee _character)
          (Movement|ProcessInputasRotation _character DeltaSeconds)
          (else
            (Movement|ProcessInputasMovement _character)))))))

(event EventPossess
  (params (PossessedPawn :type Pawn%20Object%20Reference))
  (Utilities|FlowControl|Sequence
    (:then_0
      (Utilities|FlowControl|DoOnce false
        (:Completed
          (CallFunction|CreateHUD))))
    (:then_1
      (CallFunction|SetHUDVisiblity true))))

(event Input|AxisEvents|InputAxisRotateCamera
  (params (AxisValue :type Float%20%28single-precision%29))
  (Class|PlayerController|AddYawInput AxisValue))

(fn ConstructionScript)

(fn SetBlockMovementInput
  (params (NewBlockInput :type Boolean))
  (Variables|Default|SetbBlockMovement NewBlockInput))

(fn ShouldProcessMovement
  (return (not (Variables|Default|GetbBlockMovement))))

(fn ProcessInputasMovement
  (params (PlayerCharacter :type BP%20Player%20Character%20Object%20Reference))
  (bind _playercameramanager (Variables|Default|GetPlayerCameraManager))
  (bind _returnvalue (Camera|GetCameraRotation _playercameramanager))
  (Pawn|Input|AddMovementInput PlayerCharacter (Math|Vector|GetForwardVector _returnvalue) (Input|AxisValues|GetMoveForward) false)
  (Pawn|Input|AddMovementInput PlayerCharacter (Math|Vector|GetRightVector _returnvalue) (Input|AxisValues|GetMoveRight) false))

(fn ProcessInputasRotation
  (params (PlayerCharacter :type BP%20Player%20Character%20Object%20Reference) (FrameDeltaTime :type Float%20%28single-precision%29))
  (bind _returnvalue (Input|AxisValues|GetMoveForward))
  (bind _returnvalue_2 (Input|AxisValues|GetMoveRight))
  (bind _returnvalue_3 (Math|Vector|MakeVector _returnvalue _returnvalue_2 0.0))
  (if (> (Math|Vector|VectorLengthSquared _returnvalue_3) 0.0)
    (Transformation|SetActorRotation PlayerCharacter (Math|Rotator|Lerp(Rotator) (Transformation|GetActorRotation PlayerCharacter) (Math|Rotator|Delta(Rotator) (Math|Rotator|MakeRotfromX _returnvalue_3) (Math|Rotator|MakeRotator 0.0 0.0 (* (.yaw (Camera|GetCameraRotation (Variables|Default|GetPlayerCameraManager))) -1.0))) (* FrameDeltaTime (Variables|/Game/RPG/Player/BP_PlayerCharacter.BP_PlayerCharacter_C|GetRotateSpeed PlayerCharacter)) true))))