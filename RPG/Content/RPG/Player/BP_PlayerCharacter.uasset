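; Player character Blueprint for an RPG that binds input to melee, heal and damage abilities and feeds health to the HUD.
; On BeginPlay it grants those abilities and spawns and equips a default sword through temporary setup functions.
; Left click activates the sword ability, or tries the next combo section if melee is already active; R and T trigger heal and damage.
; Tick pushes current and max health to the player HUD every frame.
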(event EventBeginPlay
  (|CallParentFunction)
  (Class|RPGCharacterBase|TempGiveAbility (Variables|Default|GetHealAbility))
  (Class|RPGCharacterBase|TempGiveAbility (Variables|Default|GetDamageAbility))
  (Class|RPGCharacterBase|TempGiveAbility (Variables|Default|GetSwordAbility))
  (Temp|TempGiveDefaultWeapon))

(event EventTick
  (params (DeltaSeconds :type Float%20%28single-precision%29))
  (Default|SetHP (Variables|/Game/RPG/Player/BP_PlayerController.BP_PlayerController_C|GetPlayerHUD (CallFunction|GetRPGPlayerController self)) (Class|RPGCharacterBase|GetHealth) (Class|RPGCharacterBase|GetMaxHealth)))

(event Input|MouseEvents|LeftMouseButton
  (params (Key :type Key%20Structure))
  (:Pressed
    (CallFunction|DoMeleeAttack)))

(event Input|KeyboardEvents|R
  (params (Key :type Key%20Structure))
  (:Pressed
    (Class|RPGCharacterBase|ActivateAbility (Variables|Default|GetHealAbility) true)))

(event Input|KeyboardEvents|T
  (params (Key :type Key%20Structure))
  (:Pressed
    (Class|RPGCharacterBase|ActivateAbility (Variables|Default|GetDamageAbility) true)))

(fn ConstructionScript)

(fn DoMeleeAttack
  (if (CallFunction|IsUsingMelee)
    (CallFunction|TryJumptoNextComboSection)
    (else
      (Class|RPGCharacterBase|ActivateAbility (Variables|Default|GetSwordAbility) true))))

(fn TempGiveDefaultWeapon
  (bind _returnvalue (Game|SpawnActorfromClass "/Game/RPG/Weapons/BP_Weapon_SwordBlackNight.BP_Weapon_SwordBlackNight_C" (Math|Transform|MakeTransform "0, 0, 0") "AlwaysSpawn" self 0))
  (CallFunction|EquipWeapon _returnvalue))