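; Black Night sword weapon Blueprint that extends its parent's equip logic with auxiliary weapons for jump slam and chest kick.
; After the parent equip runs, it spawns a bare-hands jump slam actor and a bare-foot actor, reusing existing ones when valid.
; Each is snapped to the new owner's right hand or right foot socket and has its owner set to that character.
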(event EventEquiptoOwner
  (params (NewOwner :type BP%20Character%20Object%20Reference) (SocketName :type Name :default "None"))
  (|CallParentFunction NewOwner SocketName)
  (CallFunction|AttachJumpSlamWeapon NewOwner)
  (CallFunction|AttachChestKickWeapon NewOwner))

(fn ConstructionScript
  (|CallParentFunction))

(fn AttachJumpSlamWeapon
  (params (NewOwner :type BP%20Character%20Object%20Reference))
  (Utilities|IsValid (Variables|Default|GetJumpSlamWeapon)
    (:Is%20Valid
      _)
    (:Is%20Not%20Valid
      (bind _returnvalue (Game|SpawnActorfromClass "/Game/RPG/Weapons/BP_BareHands_JumpSlam.BP_BareHands_JumpSlam_C" (Math|Transform|MakeTransform "0, 0, 0") "AlwaysSpawn" 0 0))
      (Variables|Default|SetJumpSlamWeapon _returnvalue)))
  (Transformation|AttachComponentToComponent (Variables|Default|GetJumpSlamWeapon) (Variables|/Script/Engine.Character|GetMesh NewOwner) (Variables|/Game/RPG/Core/BP_Character.BP_Character_C|GetSocket_HandRight NewOwner) "SnapToTarget" "SnapToTarget" "KeepWorld" true)
  (Actor|SetOwner (Variables|Default|GetJumpSlamWeapon) NewOwner))

(fn AttachChestKickWeapon
  (params (NewOwner :type BP%20Character%20Object%20Reference))
  (Utilities|IsValid (Variables|Default|GetChestKickWeapon)
    (:Is%20Valid
      _)
    (:Is%20Not%20Valid
      (bind _returnvalue (Game|SpawnActorfromClass "/Game/RPG/Weapons/BP_BareFoot.BP_BareFoot_C" (Math|Transform|MakeTransform "0,0.000000, 0") "AlwaysSpawn" 0 0))
      (Variables|Default|SetChestKickWeapon _returnvalue)))
  (Transformation|AttachComponentToComponent (Variables|Default|GetChestKickWeapon) (Variables|/Script/Engine.Character|GetMesh NewOwner) (Variables|/Game/RPG/Core/BP_Character.BP_Character_C|GetSocket_FootRight NewOwner) "SnapToTarget" "SnapToTarget" "KeepWorld" true)
  (Actor|SetOwner (Variables|Default|GetChestKickWeapon) NewOwner))