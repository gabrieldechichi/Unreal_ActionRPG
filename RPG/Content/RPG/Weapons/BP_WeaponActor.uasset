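; Weapon actor that snaps to an owner's mesh socket and detects melee hits on RPG characters.
; BeginAttack checks the attack tag against AcceptTags and enables query-only capsule collision; EndAttack clears both tag and collision.
; Overlapping another RPGCharacterBase sends the current tag as a gameplay event to the owner, with the target in the payload.
; Each hit also triggers a short, delayed global time-dilation hit pause.
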(event OnComponentBeginOverlap(CapsuleCollision)
  (params (OverlappedComponent :type Primitive%20Component%20Object%20Reference) (OtherActor :type Actor%20Object%20Reference) (OtherComp :type Primitive%20Component%20Object%20Reference) (OtherBodyIndex :type Integer) (bFromSweep :type Boolean) (SweepResult :type Hit%20Result%20Structure%20%28by%20ref%29))
  (if (and (!= OtherActor (Components|GetOwner)) (Utilities|ClassIsChildOf (Utilities|GetClass OtherActor) "/Script/RPG.RPGCharacterBase"))
    (Ability|SendGameplayEventtoActor (Components|GetOwner) (Variables|Default|GetCurrentAttackTag) (Utilities|Struct|MakeGameplayEventData "" (Components|GetOwner) OtherActor))
    (CallFunction|HitPause)))

(event Custom|HitPause
  (Utilities|FlowControl|Delay 0.1)
  (Utilities|Time|SetGlobalTimeDilation 0.1)
  (Utilities|FlowControl|Delay 0.01)
  (Utilities|Time|SetGlobalTimeDilation 1.0))

(fn ConstructionScript)

(fn BeginAttack
  (params (AttackTag :type Gameplay%20Tag%20Structure))
  (if (CallFunction|CanBeginAttack AttackTag)
    (Variables|Default|SetCurrentAttackTag AttackTag)
    (Collision|SetCollisionEnabled (Variables|Default|GetCapsuleCollision) "QueryOnly")))

(fn EndAttack
  (Variables|Default|SetCurrentAttackTag "")
  (Collision|SetCollisionEnabled (Variables|Default|GetCapsuleCollision) "NoCollision"))

(fn EquiptoOwner
  (params (NewOwner :type BP%20Character%20Object%20Reference) (SocketName :type Name))
  (Transformation|AttachComponentToComponent (Variables|/Script/Engine.Character|GetMesh NewOwner) SocketName "SnapToTarget" "SnapToTarget" "KeepWorld" true)
  (Actor|SetOwner self NewOwner)
  (Collision|SetCollisionEnabled (Variables|Default|GetCapsuleCollision) "NoCollision")
  (Rendering|SetActorHiddenInGame false))

(fn UnnequipfromOwner
  (Transformation|DetachFromActor "KeepWorld" "KeepWorld" "KeepWorld")
  (Rendering|SetActorHiddenInGame true))

(fn CanBeginAttack
  (params (AttackTag :type Gameplay%20Tag%20Structure))
  (if (GameplayTags|HasTag (Variables|Default|GetAcceptTags) AttackTag)
    (return true)
    (else
      (Development|PrintString (Utilities|String|ToString(Text) (Utilities|Text|FormatText "Error: Couldn't begin attack for Weapon {WeaponName}. Received tag {ReceivedTag}" (Utilities|Text|ToText(String) (Utilities|GetDisplayName self)) (Utilities|Text|ToText(Name) (GameplayTags|GetTagName AttackTag)))) true true "(R=1.000000,G=0.000000,B=0.000000,A=1.000000)")
      (return false))))