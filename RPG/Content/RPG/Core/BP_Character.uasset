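; BP_Character is an RPG character Blueprint that provides weapon equipping and melee combo helpers on top of gameplay abilities.
; A queued section name and gate flag let TryJumpToNextComboSection chain the active montage into the next combo section, then reset both.
; EquipWeapon unequips the current weapon before attaching the new one to the right-hand socket.
; IsUsingMelee checks for active Ability.Melee abilities, while IsDead is a stub returning false.
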(event EventBeginPlay)

(event Collision|EventActorBeginOverlap
  (params (OtherActor :type Actor%20Object%20Reference)))

(event EventTick
  (params (DeltaSeconds :type Float%20%28single-precision%29)))

(fn ConstructionScript)

(fn IsDead
  (return false))

(fn TryJumptoNextComboSection
  (bind _mesh (Variables|Character|GetMesh))
  (bind _returnvalue (Components|SkeletalMesh|GetAnimInstance _mesh))
  (bind _returnvalue_2 (Animation|Montage|GetCurrentActiveMontage _returnvalue))
  (if (and (Utilities|Name|NotEqual(Name) (Variables|Default|GetNextComboSection) "None") (Variables|Default|GetCanGoToNextComboSection))
    (Class|AnimInstance|MontageSetNextSection _returnvalue (Animation|Montage|MontageGetCurrentSection _returnvalue _returnvalue_2) (Variables|Default|GetNextComboSection) _returnvalue_2)
    (Combo|ResetNextComboSectionName)))

(fn SetNextComboSectionName
  (params (NextComboSectionName :type Name))
  (Variables|Default|SetNextComboSection NextComboSectionName)
  (Variables|Default|SetCanGoToNextComboSection true))

(fn ResetNextComboSectionName
  (Variables|Default|SetNextComboSection "None")
  (Variables|Default|SetCanGoToNextComboSection false))

(fn IsUsingMelee
  (return (> (Utilities|Array|Length (Class|RPGCharacterBase|GetActiveAbilitieswithTags "(GameplayTags=((TagName=\"Ability.Melee\")))")) 0)))

(fn EquipWeapon
  (params (NewWeapon :type BP%20Weapon%20Actor%20Object%20Reference))
  (Weapon|UnequipCurrentWeapon)
  (Default|EquiptoOwner NewWeapon self (Variables|Melee|GetSocket_HandRight))
  (Variables|Weapon|SetCurrentWeapon NewWeapon))

(fn UnequipCurrentWeapon
  (Utilities|IsValid (Variables|Weapon|GetCurrentWeapon)
    (:Is%20Valid
      (Default|UnnequipfromOwner (Variables|Weapon|GetCurrentWeapon))
      (Variables|Weapon|SetCurrentWeapon 0))))